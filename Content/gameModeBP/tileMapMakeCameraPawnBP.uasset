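; Camera pawn for the tile map maker, as its name suggests, that moves freely through world space.
; Holding the right mouse button enables inverted mouse-drag panning in X and Y, while keyboard axes pan directly and a Lift axis changes height.
; Every move is an unswept world offset with a fixed per-axis speed and no delta-time scaling.
; The construction script resets the pawn to a fixed elevated position above the world origin.
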(event `Key|RightMouseButton`
  (params (Key :type "Key Structure"))
  ;[1 1 1] 获得鼠标左键状态
  (:`Pressed`
    (set `self.isMouseRightPress` true))
  (:`Released`
    (set `self.isMouseRightPress` false)))

(event `InputAxis|XMOuse`
  (params (AxisValue :type "Float (single-precision)"))
  (if (`self.isMouseRightPress`)
    (`self.K2_AddActorWorldOffset` (`KismetMathLibrary.MakeVector` 0.0 (* AxisValue -30.0)))))

(event `InputAxis|Xkeyboard`
  (params (AxisValue :type "Float (single-precision)"))
  (`self.K2_AddActorWorldOffset` (`KismetMathLibrary.MakeVector` 0.0 (* AxisValue 40.0))))

(event `InputAxis|YMouse`
  (params (AxisValue :type "Float (single-precision)"))
  (if (`self.isMouseRightPress`)
    (`self.K2_AddActorWorldOffset` (`KismetMathLibrary.MakeVector` (* AxisValue -30.0)))))

(event `InputAxis|Ykeyboard`
  (params (AxisValue :type "Float (single-precision)"))
  (`self.K2_AddActorWorldOffset` (`KismetMathLibrary.MakeVector` (* AxisValue 40.0))))

(event `InputAxis|Lift`
  (params (AxisValue :type "Float (single-precision)"))
  (`self.K2_AddActorWorldOffset` (`KismetMathLibrary.MakeVector` 0.0 0.0 (* AxisValue 50.0))))

(fn `UserConstructionScript`
  (`self.K2_SetActorLocationAndRotation` (0.0 0.0 500.0)))